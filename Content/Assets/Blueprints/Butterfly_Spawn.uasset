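; Butterfly spawner that adds butterflies to the level in response to the player's meditation level from an OpenViBE signal.
; On BeginPlay it opens an OpenViBE signal listener and caches the transforms of all Spawn_Localization actors.
; Tick reads the meditation channel and uses a Delay to throttle spawn checks.
; A high enough value spawns a BP_Butterfly at a randomly picked cached location, until a counter reaches its cap.
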(event EventBeginPlay
  (bind _openvibeinterface (Variables|Default|GetOpenVibeInterface))
  (Class|OpenVibeInterfaceComponent|ActivateOpenVibeInterface _openvibeinterface)
  (Class|OpenVibeInterfaceComponent|AddDataListener _openvibeinterface "Signal" 5678)
  ;[1 1 1] Get all Spawn Localizations
  (bind _outactors (Actor|GetAllActorsOfClass "/Game/Assets/Blueprints/Spawn_Localization.Spawn_Localization_C"))
  (for _array_element _outactors
    (bind _returnvalue (Utilities|Array|Add (Variables|Default|GetLocalizations) (Transformation|GetWorldTransform (Variables|/Game/Assets/Blueprints/Spawn_Localization.Spawn_Localization_C|GetDefaultSceneRoot _array_element))))
    (Variables|Default|SetArray%20size _returnvalue)))

(event EventTick
  (params (DeltaSeconds :type Float%20%28single-precision%29))
  (bind _output_get (Variables|Default|SetMeditation (Class|OpenVibeInterfaceComponent|GetSignalValue (Variables|Default|GetOpenVibeInterface) 0 2)))
  (Utilities|FlowControl|Delay 1e+01)
  (if (and (>= _output_get 5e+01) (<= (Variables|Default|Getbutterfly%20count) 10))
    (Game|SpawnActorfromClass "/Game/Assets/Blueprints/BP_Butterfly.BP_Butterfly_C" (Utilities|Array|Get(acopy) (Variables|Default|GetLocalizations) (Math|Random|RandomInteger (Variables|Default|GetArray%20size))) "Undefined" 0 0)
    (Math|Integer|IncrementInt (Variables|Default|Getbutterfly%20count))))

(fn ConstructionScript)